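; BP_Tower is a level 2 tower that brightens and tracks the player's crystal progress toward a win.
; At BeginPlay it creates and stores a dynamic material instance on its Tower component.
; Its Brighten event raises the material's Emissive parameter a step, increments the Crystals count on BP_ThirdPersonCharacter, and prints a win message when the count reaches three.
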(event `self.ReceiveBeginPlay`
  (bind _returnvalue (`PrimitiveComponent.CreateDynamicMaterialInstance` (`self.tower`) 0 "/Game/Mesh/Material_001.Material_001" "None"))
  (set `self.TowerMaterial` _returnvalue))

(event `Brighten`
  (bind _towermaterial (`self.TowerMaterial`))
  (bind _returnvalue (`MaterialInstanceDynamic.K2_GetScalarParameterValue` _towermaterial "Emissive"))
  (`MaterialInstanceDynamic.SetScalarParameterValue` _towermaterial "Emissive" (+ _returnvalue 0.15))
  (bind _asbp_third_person_character (cast `/Game/ThirdPerson/Blueprints/BP_ThirdPersonCharacter` (`GameplayStatics.GetPlayerCharacter` 0)))
  (bind _output_get (set `/Game/ThirdPerson/Blueprints/BP_ThirdPersonCharacter.Crystals` (+ 1 (`/Game/ThirdPerson/Blueprints/BP_ThirdPersonCharacter.Crystals` _asbp_third_person_character)) _asbp_third_person_character))
  (if (== _output_get 3)
    (`KismetSystemLibrary.PrintString` "WIN")
    (else
      (`KismetSystemLibrary.PrintString` "not yet"))))

(fn `UserConstructionScript`)