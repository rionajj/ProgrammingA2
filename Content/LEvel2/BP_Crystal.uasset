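; BP_Crystal is a rotating level crystal that, on overlap, plays a collection effect and brightens a Tower.
; Its own actor tag (Crystal1, Crystal2 or Crystal3) selects which Level Sequence plays.
; Box overlap attaches a spline-follow Niagara system to the crystal, starts that sequence and disables box collision to prevent retriggering.
; After a delay specific to each crystal, it calls Brighten on the Tower.
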(event `self.ReceiveBeginPlay`
  (`AddComponent|NODE_AddRotatingMovementComponent-0`)
  (set `self.1` "Crystal1")
  (set `self.2` "Crystal2")
  (set `self.3` "Crystal3")
  (set `self.Splineee` null))

(event `self.Box.OnComponentBeginOverlap`
  (params (OverlappedComponent :type "PrimitiveComponent Object Reference") (OtherActor :type "Actor Object Reference") (OtherComp :type "PrimitiveComponent Object Reference") (OtherBodyIndex :type Integer) (bFromSweep :type Boolean) (SweepResult :type "HitResult Structure (by ref)"))
  (if (`self.ActorHasTag` (`self.3`))
    (`NiagaraFunctionLibrary.SpawnSystemAttached` "/Game/_SplineVFX/NS/NS_Spline_ParticleFollow.NS_Spline_ParticleFollow" (`self.Crystal`) "None" (0.0 0.0 0.0) (struct) "SnapToTarget")
    (bind (_outactor _returnvalue) (`LevelSequencePlayer.CreateLevelSequencePlayer` "/Game/LEvel2/Sequence_Crystal3.Sequence_Crystal3"))
    (`MovieSceneSequencePlayer.Play` _returnvalue)
    (`PrimitiveComponent.SetCollisionEnabled` (`self.Box`) "NoCollision")
    (`KismetSystemLibrary.Delay` 1.5)
    (`/Game/LEvel2/BP_Tower.Brighten` (`self.Tower`))
    (elif (`self.ActorHasTag` (`self.2`))
      (`NiagaraFunctionLibrary.SpawnSystemAttached` "/Game/_SplineVFX/NS/NS_Spline_ParticleFollow.NS_Spline_ParticleFollow" (`self.Crystal`) "None" (0.0 0.0 0.0) (struct) "SnapToTarget")
      (bind (_outactor_2 _returnvalue_2) (`LevelSequencePlayer.CreateLevelSequencePlayer` "/Game/LEvel2/Sequence_Crystal2.Sequence_Crystal2"))
      (`MovieSceneSequencePlayer.Play` _returnvalue_2)
      (`PrimitiveComponent.SetCollisionEnabled` (`self.Box`) "NoCollision")
      (`KismetSystemLibrary.Delay` 1.8)
      (`/Game/LEvel2/BP_Tower.Brighten` (`self.Tower`))
      (elif (`self.ActorHasTag` (`self.1`))
        (`NiagaraFunctionLibrary.SpawnSystemAttached` "/Game/_SplineVFX/NS/NS_Spline_ParticleFollow.NS_Spline_ParticleFollow" (`self.Crystal`) "None" (0.0 0.0 0.0) (struct) "SnapToTarget")
        (bind (_outactor_3 _returnvalue_3) (`LevelSequencePlayer.CreateLevelSequencePlayer` "/Game/LEvel2/Sequence_Crystal1.Sequence_Crystal1"))
        (`MovieSceneSequencePlayer.Play` _returnvalue_3)
        (`PrimitiveComponent.SetCollisionEnabled` (`self.Box`) "NoCollision")
        (`KismetSystemLibrary.Delay` 2.1)
        (`/Game/LEvel2/BP_Tower.Brighten` (`self.Tower`))))))

(fn `UserConstructionScript`)