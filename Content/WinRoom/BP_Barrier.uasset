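; BP_Barrier is a win-room barrier that opens in a staged magic-and-explosion sequence once unlocked.
; An external OPEN event plays a victory sound, reveals a spotlight and sign, and arms the Box trigger, which starts disabled.
; Any overlap disarms the trigger and runs a Delay-timed sequence: embers at two target actors, then an electric blast at a third.
; The Plane then loses visibility and collision, effects stop, and cheers play.
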(event `OPEN`
  (`GameplayStatics.PlaySoundAtLocation` "/Game/Sound/Sound_Victory.Sound_Victory" (`self.K2_GetActorLocation` (`GameplayStatics.GetPlayerCharacter` 0)) (struct) 0.7 1.0 0.0 null null null null)
  (`SceneComponent.SetHiddenInGame` (`self.SpotLight`) false false)
  (`SceneComponent.SetHiddenInGame` (`self.Sign`) false false)
  (`PrimitiveComponent.SetCollisionEnabled` (`self.Box`) "QueryOnly"))

(event `self.ReceiveBeginPlay`
  (`PrimitiveComponent.SetCollisionEnabled` (`self.Box`) "NoCollision"))

(event `self.Box.OnComponentBeginOverlap`
  (params (OverlappedComponent :type "PrimitiveComponent Object Reference") (OtherActor :type "Actor Object Reference") (OtherComp :type "PrimitiveComponent Object Reference") (OtherBodyIndex :type Integer) (bFromSweep :type Boolean) (SweepResult :type "HitResult Structure (by ref)"))
  (bind _returnvalue (`self.K2_GetActorLocation` (`self.TargetSpark`)))
  (`PrimitiveComponent.SetCollisionEnabled` (`self.Box`) "NoCollision")
  (`SceneComponent.SetVisibility` (`self.Sign`) false false)
  (bind _returnvalue_2 (`GameplayStatics.SpawnSoundAtLocation` "/Game/Sound/Sound_magic.Sound_magic" (0.0 0.0 0.0) (struct) 0.7 1.0 0.0 null null))
  (bind _returnvalue_3 (`GameplayStatics.SpawnEmitterAtLocation` "/Game/Realistic_Starter_VFX_Pack_Vol2/Particles/Sparks/P_Embers_A.P_Embers_A" (`self.K2_GetActorLocation` (`self.TargetEnvironment1`)) (struct) (2.0 2.0 2.0)))
  (bind _returnvalue_4 (`GameplayStatics.SpawnEmitterAtLocation` "/Game/Realistic_Starter_VFX_Pack_Vol2/Particles/Sparks/P_Embers_A.P_Embers_A" (`self.K2_GetActorLocation` (`self.TargetEnvironment2`)) (struct) (2.0 2.0 2.0)))
  (`KismetSystemLibrary.Delay` 5.0)
  (`GameplayStatics.SpawnEmitterAtLocation` "/Game/Realistic_Starter_VFX_Pack_Vol2/Particles/Destruction/P_Destruction_Electric.P_Destruction_Electric" _returnvalue (struct) (20.0 20.0 20.0))
  (bind _returnvalue_5 (`GameplayStatics.SpawnSoundAtLocation` "/Game/Sound/Sound_explosion.Sound_explosion" _returnvalue (struct) 0.9 1.0 4.9 null null))
  (`KismetSystemLibrary.Delay` 0.4)
  (`SceneComponent.SetVisibility` (`self.Plane`) false false)
  (`AudioComponent.Stop` _returnvalue_2)
  (`ActorComponent.Deactivate` _returnvalue_3)
  (`ActorComponent.Deactivate` _returnvalue_4)
  (`PrimitiveComponent.SetCollisionEnabled` (`self.Plane`) "NoCollision")
  (`KismetSystemLibrary.Delay` 2.0)
  (`AudioComponent.Stop` _returnvalue_5)
  (`KismetSystemLibrary.Delay` 0.4)
  (`GameplayStatics.PlaySoundAtLocation` "/Game/Sound/Sound_Cheers.Sound_Cheers" (0.0 0.0 0.0) (struct) 0.8 1.0 0.0 null null null null))

(fn `UserConstructionScript`)