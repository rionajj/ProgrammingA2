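; BP_Button is a button actor that spawns a temporary BP_Platforms actor when its ButtonClick event fires.
; The event disables the button's collision, spawns the platforms at the transform of the referenced SpawnLocation actor and plays a timer sound at the player character's location.
; After a fixed delay it destroys the spawned platforms and restores the button's collision for reuse.
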(event `/Game/Platforms/BPI_Interaction.ButtonClick`
  (`PrimitiveComponent.SetCollisionEnabled` (`self.Button`) "NoCollision")
  (bind _returnvalue (`|SpawnActorFromClass` "/Game/Platforms/BP_Platforms.BP_Platforms_C" (`self.GetTransform` (`self.SpawnLocation`)) "Undefined" "MultiplyWithRoot" null null))
  (`GameplayStatics.PlaySoundAtLocation` "/Game/Sound/Sound_timer.Sound_timer" (`self.K2_GetActorLocation` (`GameplayStatics.GetPlayerCharacter` 0)) (struct) 0.75 1.0 0.0 null null null null)
  (`KismetSystemLibrary.Delay` 15.0)
  (`self.K2_DestroyActor` _returnvalue)
  (`PrimitiveComponent.SetCollisionEnabled` (`self.Button`) "QueryAndPhysics"))

(fn `UserConstructionScript`)