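; Locked double door for Level 3 that needs a key before it opens.
; Overlapping its box calls Unlock on the referenced BP_Key when the Key flag is set, otherwise shows a message for two seconds.
; A separate OpenAnim event, not called within this Blueprint, plays a timeline that swings both leaves a quarter turn in opposite directions.
; Key resets to false on BeginPlay and is never set true here.
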(event `self.ReceiveBeginPlay`
  (set `self.Key?` false))

(event `self.Box.OnComponentBeginOverlap`
  (params (OverlappedComponent :type "PrimitiveComponent Object Reference") (OtherActor :type "Actor Object Reference") (OtherComp :type "PrimitiveComponent Object Reference") (OtherBodyIndex :type Integer) (bFromSweep :type Boolean) (SweepResult :type "HitResult Structure (by ref)"))
  (bind _message (`self.Message`))
  (if (`self.Key?`)
    (bind _asbp_key (cast `/Game/Level3/BP_Key` (`self.KeyBP`)))
    (`/Game/Level3/BP_Key.Unlock` _asbp_key)
    (else
      (`SceneComponent.SetHiddenInGame` _message false false)
      (`KismetSystemLibrary.Delay` 2.0)
      (`SceneComponent.SetHiddenInGame` _message true false))))

(event `OpenAnim`
  (bind (_direction _z_rotation) (`Timeline|Opening`)
    (:`Update`
      (`SceneComponent.K2_SetRelativeRotation` (`self.Door1`) (`KismetMathLibrary.MakeRotator` 0.0 0.0 (`KismetMathLibrary.Lerp` 0.0 90.0 _z_rotation)) false false)
      (`SceneComponent.K2_SetRelativeRotation` (`self.Door2`) (`KismetMathLibrary.MakeRotator` 0.0 0.0 (`KismetMathLibrary.Lerp` 0.0 -90.0 _z_rotation)) false false))))

(fn `UserConstructionScript`)