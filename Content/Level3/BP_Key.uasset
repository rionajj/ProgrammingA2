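; BP_Key is a rotating key pickup that unlocks and opens its linked BP_Door.
; Overlapping its box plays a sound, hides the key, disables collision and sets the door's Key flag.
; Unlock shows and rescales the key, stops rotation, and runs raise, insert and turn timelines, each started from the previous one's Update.
; Sounds accompany the motion, and after a delay the turn update destroys the actor and calls the door's OpenAnim.
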(event `self.ReceiveBeginPlay`
  (bind _returnvalue (`AddComponent|NODE_AddRotatingMovementComponent-0`)))

(event `self.Box.OnComponentBeginOverlap`
  (params (OverlappedComponent :type "PrimitiveComponent Object Reference") (OtherActor :type "Actor Object Reference") (OtherComp :type "PrimitiveComponent Object Reference") (OtherBodyIndex :type Integer) (bFromSweep :type Boolean) (SweepResult :type "HitResult Structure (by ref)"))
  (`GameplayStatics.SpawnSoundAttached` "/Game/Sound/Sound3/Sound_Key.Sound_Key" (`self.Key`) "None" (0.0 0.0 0.0) (struct) "KeepRelativeOffset" false 1.0 1.0 0.0 null null)
  (`SceneComponent.SetVisibility` (`self.Key`) false false)
  (`PrimitiveComponent.SetCollisionEnabled` (`self.Box`) "NoCollision")
  (bind _asbp_door (cast `/Game/Level3/BP_Door` (`self.Door`)))
  (set `/Game/Level3/BP_Door.Key?` true _asbp_door))

(event `Unlock`
  (bind (_returnvalue_x _returnvalue_y _returnvalue_z) (`KismetMathLibrary.BreakVector` (`self.K2_GetActorLocation`)))
  (bind _key (`self.Key`))
  (bind (_returnvalue_x_2 _returnvalue_y_2) (`KismetMathLibrary.BreakVector` (`self.K2_GetActorLocation` (`self.UnlockPoint`))))
  (`SceneComponent.SetVisibility` (`self.Key`) true false)
  (`ActorComponent.SetComponentTickEnabled` (stale `self.ReceiveBeginPlay` _returnvalue) false)
  (`SceneComponent.SetRelativeScale3D` _key (0.005 0.005 0.005))
  (bind (_direction _z_position) (`Timeline|KeyRaise` :!via `PlayFromStart`)
    (:`Update`
      (`SceneComponent.K2_SetWorldLocationAndRotation` :`self` _key :`NewLocation` (`KismetMathLibrary.MakeVector` _returnvalue_x_2 _returnvalue_y_2 (`KismetMathLibrary.Lerp` 7330.0 7410.0 _z_position)) :`bTeleport` true)
      (bind (_direction_2 _y_position) (`Timeline|KeyIn` :!via `PlayFromStart`)
        (:`Update`
          (`self.K2_SetActorLocation` (`KismetMathLibrary.MakeVector` _returnvalue_x (`KismetMathLibrary.Lerp` 6970.0 7230.0 _y_position) _returnvalue_z))
          (bind (_direction_3 _y_rotation) (`Timeline|KeyTurn` :!via `PlayFromStart`)
            (:`Update`
              (`SceneComponent.K2_SetWorldRotation` (`self.Key`) (`KismetMathLibrary.MakeRotator` (`KismetMathLibrary.Lerp` 0.0 -90.0 _y_rotation) 0.0 -90.0) false false)
              (`KismetSystemLibrary.Delay` 1.5)
              (`self.K2_DestroyActor`)
              (bind _asbp_door (cast `/Game/Level3/BP_Door` (`self.Door`)))
              (`/Game/Level3/BP_Door.OpenAnim` _asbp_door))
            (:`Finished`
              (`GameplayStatics.SpawnSoundAtLocation` "/Game/Sound/Sound3/Sound_door.Sound_door" (0.0 0.0 0.0) (struct) 1.0 1.0 4.0 null null))))
        (:`Finished`
          (`GameplayStatics.SpawnSoundAtLocation` "/Game/Sound/Sound3/Sound_click.Sound_click" (0.0 0.0 0.0) (struct) 1.0 1.0 0.0 null null)
          (`KismetSystemLibrary.Delay` 0.2)
          (`GameplayStatics.SpawnSoundAtLocation` "/Game/Sound/Sound3/Sound_unlock.Sound_unlock" (0.0 0.0 0.0) (struct) 1.0 1.0 0.0 null null))))))

(fn `UserConstructionScript`)